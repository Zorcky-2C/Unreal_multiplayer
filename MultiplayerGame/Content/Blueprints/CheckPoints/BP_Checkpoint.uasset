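; BP_Checkpoint is a checkpoint trigger that updates a character's respawn point and can act as the goal that ends the game.
; When a ThirdPersonCharacter overlaps its Box, it passes the world transform of TargetSpawnLoc to that character as the respawn transform.
; If IsItLastCheckPoint is set, it also marks the character as winner, destroys the Box and shows the WB_EndGame widget.
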(event OnComponentBeginOverlap(Box)
  (params (OverlappedComponent :type Primitive%20Component%20Object%20Reference) (OtherActor :type Actor%20Object%20Reference) (OtherComp :type Primitive%20Component%20Object%20Reference) (OtherBodyIndex :type Integer) (bFromSweep :type Boolean) (SweepResult :type Hit%20Result%20Structure%20%28by%20ref%29))
  ;[1 1 1 1 50] Set the new respawn point for the players - check if this is the last checkpoint and the goal of the current game
  (bind _asthird_person_character (Utilities|Casting|CastToThirdPersonCharacter OtherActor))
  (Default|SetRespawnTransform _asthird_person_character (Transformation|GetWorldTransform (Variables|Default|GetTargetSpawnLoc)))
  (if (Variables|Default|GetIsItLastCheckPoint?)
    (Default|SetHasWon _asthird_person_character true)
    (Components|DestroyComponent (Variables|Default|GetBox))
    (bind _returnvalue (UserInterface|CreateWidget "/Game/Blueprints/Widget/WB_EndGame.WB_EndGame_C"))
    (UserInterface|Viewport|AddtoViewport _returnvalue 0)))

(fn ConstructionScript)